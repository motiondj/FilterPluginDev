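; Test actor that compares Kalman and One Euro vector filters on a noisy moving position.
; Each Tick builds an orbit-and-bob point from TestTime, which this graph never advances, adds random noise, then runs both filters on it.
; Three small meshes show raw and filtered results at world positions, with the filtered ones offset sideways on Y.
; Color-coded on-screen text prints each position for comparison.
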(event `self.ReceiveTick`
  (params (DeltaSeconds :type "Float (single-precision)"))
  (bind _output_get (set `self.RawPosition` (+ (`KismetMathLibrary.MakeVector` (* (`KismetMathLibrary.Cos` (* (`self.TestTime`) (`self.OrbitSpeed`))) (`self.OrbitRadius`)) (* (`KismetMathLibrary.Sin` (* (`self.TestTime`) (`self.OrbitSpeed`))) (`self.OrbitRadius`)) (* (`KismetMathLibrary.Sin` (* (`self.TestTime`) 2.0)) 50.0)) (* (`KismetMathLibrary.RandomUnitVectorInConeInDegrees` (1.0 1.0 1.0) 180.0) (`self.NoiseIntensity`)))))
  (bind _returnvalue (`FilterBPLibrary.KalmanFilterVector` _output_get "Medium" "VectorKalman"))
  (set `self.KalmanPosition` _returnvalue)
  (bind _returnvalue_2 (`FilterBPLibrary.OneEuroFilterVector` (`self.RawPosition`) DeltaSeconds "Medium" "VectorOneEuro"))
  (set `self.OneEuroPosition` _returnvalue_2)
  (`self.Cube Location`)
  (`self.output_Event`))

(event `Cube Location`
  (`SceneComponent.K2_SetWorldLocation` (`self.RawMesh`) (`self.RawPosition`) false false)
  (`SceneComponent.K2_SetWorldLocation` (`self.KalmanMesh`) (+ (`self.KalmanPosition`) (0.0 50.0 0.0)) false false)
  (`SceneComponent.K2_SetWorldLocation` (`self.OneEuroMesh`) (+ (`self.OneEuroPosition`) (0.0 -50.0 0.0)) false false))

(event `output_Event`
  (bind (_rawposition_x _rawposition_y _rawposition_z) (`KismetMathLibrary.BreakVector` (`self.RawPosition`)))
  (bind (_kalmanposition_x _kalmanposition_y _kalmanposition_z) (`KismetMathLibrary.BreakVector` (`self.KalmanPosition`)))
  (bind (_oneeuroposition_x _oneeuroposition_y _oneeuroposition_z) (`KismetMathLibrary.BreakVector` (`self.OneEuroPosition`)))
  (`KismetSystemLibrary.PrintString` (`KismetTextLibrary.Conv_TextToString` (`|FormatText` "Raw: X={0:.1f} Y={1:.1f} Z={2:.1f}" _rawposition_x _rawposition_y _rawposition_z)) true true (struct :`R` 1.0 :`A` 1.0) 0.0)
  (`KismetSystemLibrary.PrintString` (`KismetTextLibrary.Conv_TextToString` (`|FormatText` "Kalman: X={0:.1f} Y={1:.1f} Z={2:.1f}" _kalmanposition_x _kalmanposition_y _kalmanposition_z)) true true (struct :`G` 1.0 :`A` 1.0) 0.0)
  (`KismetSystemLibrary.PrintString` (`KismetTextLibrary.Conv_TextToString` (`|FormatText` "OneEuro: X={0:.1f} Y={1:.1f} Z={2:.1f}" _oneeuroposition_x _oneeuroposition_y _oneeuroposition_z)) true true (struct :`B` 1.0 :`A` 1.0) 0.0))

(fn `UserConstructionScript`
  (`SceneComponent.K2_SetWorldTransform` (`self.RawMesh`) (`KismetMathLibrary.MakeTransform` (0.0 0.0 0.0) (struct) (0.2 0.2 0.2)) false false)
  (`SceneComponent.K2_SetWorldTransform` (`self.KalmanMesh`) (`KismetMathLibrary.MakeTransform` (0.0 50.0 0.0) (struct) (0.2 0.2 0.2)) false false)
  (`SceneComponent.K2_SetWorldTransform` (`self.OneEuroMesh`) (`KismetMathLibrary.MakeTransform` (0.0 -50.0 0.0) (struct) (0.2 0.2 0.2)) false false))