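; Test actor that exercises a signal-filter library's custom presets, weighted filter chains and profiling.
; BeginPlay creates and stores a One Euro "VRController" preset, a Kalman "SmoothCamera" preset and a weighted Kalman/One Euro chain.
; Tick builds a noisy sine test signal and starts profiling, but never ends it or filters the signal.
; The nodes that apply a preset and update a filter are unconnected.
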(event `self.ReceiveBeginPlay`
  (`KismetSystemLibrary.PrintString` "Advanced Feature Test Starte")
  (bind _returnvalue (`FilterBPLibrary.CreateCustomPreset` "VRController" "OneEuro" 0.3 0.0001))
  (set `self.VRController_Preset_Ref` _returnvalue)
  (`KismetSystemLibrary.PrintString` "Custom Preset Created: VRController")
  (bind _returnvalue_2 (`FilterBPLibrary.CreateCustomPreset` "SmoothCamera" "Kalman" 0.001 2.0))
  (set `self.SmoothCamera_Preset_Ref` _returnvalue_2)
  (`KismetSystemLibrary.PrintString` "Custom Preset Created: SmoothCamera")
  (bind _returnvalue_3 (`FilterBPLibrary.CreateFilterChainWithWeights` (`|MakeArray` "Kalman" "OneEuro" :!type "EFilterType Enum") (`|MakeArray` "Medium" "Low" :!type "EFilterPreset Enum") (`|MakeArray` 0.7 0.3 :!type "Float (single-precision)")))
  (set `self.TestFilterChain` _returnvalue_3))

(event `self.ReceiveTick`
  (params (DeltaSeconds :type "Float (single-precision)"))
  (bind _output_get (set `self.TestTime` (+ (`self.TestTime`) DeltaSeconds)))
  (set `self.TestSignal` (+ (* (`KismetMathLibrary.Sin` _output_get) 100.0) (`KismetMathLibrary.RandomFloatInRange` -20.0 20.0)))
  (`FilterBPLibrary.StartProfiling` "AdvancedTest"))

(fn `UserConstructionScript`)