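; BP_OneClickMacroTest is a test actor that compares Kalman and One Euro smoothing filters on a noisy synthetic signal.
; Each Tick it builds a sine wave from accumulated time and adds random noise.
; It feeds that value through both filter calls, using High presets and string filter IDs.
; The raw and both filtered values print to screen every frame for side-by-side comparison.
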(event `self.ReceiveBeginPlay`
  (`KismetSystemLibrary.PrintString` "One-Click Macro Test Started!"))

(event `self.ReceiveTick`
  (params (DeltaSeconds :type "Float (single-precision)"))
  (bind _noiseamount (`self.NoiseAmount`))
  (bind _output_get (set `self.TestTime` (+ (`self.TestTime`) DeltaSeconds)))
  (bind _output_get_2 (set `self.RawValue` (+ (`KismetMathLibrary.Sin` (* _output_get (`self.TestFrequency`))) (`KismetMathLibrary.RandomFloatInRange` (* _noiseamount -1.0) _noiseamount))))
  (bind _returnvalue (`FilterBPLibrary.KalmanFilterValue` _output_get_2 "High" "TestKalman"))
  (bind _output_get_3 (set `self.KalmanResult` _returnvalue))
  (bind _returnvalue_2 (`FilterBPLibrary.OneEuroFilterValue` _output_get_2 DeltaSeconds "High" "TestOneEuro"))
  (bind _output_get_4 (set `self.OneEuroResult` _returnvalue_2))
  (`KismetSystemLibrary.PrintString` (`KismetTextLibrary.Conv_TextToString` (`|FormatText` "Raw: {0:.2f} | Kalman: {1:.2f} | OneEuro: {2:.2f}" _output_get_2 _output_get_3 _output_get_4)) true true (struct :`R` 1.0 :`G` 1.0 :`B` 1.0 :`A` 1.0) 0.0))

(fn `UserConstructionScript`)